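; BP_FlyingDuckCharacter is a flying duck character that travels along the path of a referenced spline.
; Each Tick it snaps its location to the world-space spline point at SplineDistance and takes its rotation from the spline's local-space rotation there.
; SplineDistance then grows by a fixed step per frame, so speed depends on frame rate, with no wrap or end check.
; Tick also feeds forward movement input before overriding the transform.
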(event EventTick
  (params (DeltaSeconds :type Float%20%28single-precision%29))
  (Pawn|Input|AddMovementInput (Transformation|GetActorForwardVector self) 1.0 false)
  (Transformation|SetActorLocation (Spline|GetLocationatDistanceAlongSpline (Variables|/Game/Blueprints/SplineBP.SplineBP_C|GetSPLINE (Variables|Default|GetSPLINE)) (Variables|Default|GetSplineDistance) "World") false false)
  (Transformation|SetActorRotation (Spline|GetRotationatDistanceAlongSpline (Variables|/Game/Blueprints/SplineBP.SplineBP_C|GetSPLINE (Variables|Default|GetSPLINE)) (Variables|Default|GetSplineDistance) "Local"))
  (Variables|Default|SetSplineDistance (+ (Variables|Default|GetSplineDistance) 3.0)))

(fn ConstructionScript)